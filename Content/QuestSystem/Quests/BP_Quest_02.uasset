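; Quest "Out in Left Field", in which the player fetches blue and orange cubes and delivers them to Manny.
; ConstructRootObjectiveCollection creates the named root collection, and PopulateObjectives adds two fetch objectives and a deliver objective to it.
; Fetch objectives receive their cube data, a name built from the amount to fetch, and the InventoryComponent cached from the player pawn on BeginPlay.
; The deliver objective receives the target actor and this quest.
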(event EventBeginPlay
  (Variables|Default|SetInventoryComponent (Actor|GetComponentbyClass (Game|Player|GetPlayerPawn 0) "/Script/QuestSystem.InventoryComponent")))

(event EventPopulateObjectives
  (params (ObjectiveCollection :type Objective%20Collection%20Object%20Reference))
  (Utilities|FlowControl|Sequence
    (:then_0
      (bind _returnvalue (Game|ConstructObjectfromClass "/Game/QuestSystem/Objectives/BP_FetchItemsObjective.BP_FetchItemsObjective_C" (Variables|Default|GetBlueCubeData) (Variables|Default|GetInventoryComponent) false (CallFunction|GetObjectiveName (Variables|Default|GetBlueCubeData) "Blue Cubes")))
      (Class|ObjectiveCollection|AddObjective (Class|QuestBase|GetRootObjectiveCollection) _returnvalue))
    (:then_1
      (bind _returnvalue_2 (Game|ConstructObjectfromClass "/Game/QuestSystem/Objectives/BP_FetchItemsObjective.BP_FetchItemsObjective_C" (Variables|Default|GetOrangeCubeData) (Variables|Default|GetInventoryComponent) false (CallFunction|GetObjectiveName (Variables|Default|GetOrangeCubeData) "Orange Cubes")))
      (Class|ObjectiveCollection|AddObjective (Class|QuestBase|GetRootObjectiveCollection) _returnvalue_2))
    (:then_2
      (bind _returnvalue_3 (Game|ConstructObjectfromClass "/Game/QuestSystem/Objectives/BP_DeliverQuestObjective.BP_DeliverQuestObjective_C" (Variables|Default|GetActor%20to%20Deliver) self false "Deliver the cubes to Manny"))
      (Class|ObjectiveCollection|AddObjective (Class|QuestBase|GetRootObjectiveCollection) _returnvalue_3))))

(fn ConstructionScript)

(fn ConstructRootObjectiveCollection
  (bind _returnvalue (Game|ConstructObjectfromClass "/Script/QuestSystem.ObjectiveCollection" false false "Out in Left Field"))
  (return _returnvalue))

(fn GetObjectiveName
  (params (FetchItemsData :type S%20Fetch%20Items%20Data%20Structure) (ObjectName :type String))
  (return (Utilities|Text|ToText(String) (Utilities|String|Append "Pick up " (Utilities|String|ToString(Integer) (.amounttofetch FetchItemsData)) " " ObjectName))))