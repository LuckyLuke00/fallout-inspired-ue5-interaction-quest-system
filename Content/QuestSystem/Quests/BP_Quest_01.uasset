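; BP_Quest_01 is a quest named "Out of Time" that sends the player to home, Concord and Diamond City.
; It overrides root collection construction to create an ordered ObjectiveCollection that disallows skipping and is itself flagged optional.
; PopulateObjectives fills that root collection with three reach-destination objectives in sequence, each bound to a trigger, with the Concord investigation marked optional.
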(event EventPopulateObjectives
  (params (ObjectiveCollection :type Objective%20Collection%20Object%20Reference))
  (Utilities|FlowControl|Sequence
    (:then_0
      (bind _returnvalue (Game|ConstructObjectfromClass "/Game/QuestSystem/Objectives/BP_ReachDestinationObjective.BP_ReachDestinationObjective_C" (Variables|Default|GetHomeTrigger) false "Go home"))
      (Class|ObjectiveCollection|AddObjective (Class|QuestBase|GetRootObjectiveCollection) _returnvalue))
    (:then_1
      (bind _returnvalue_2 (Game|ConstructObjectfromClass "/Game/QuestSystem/Objectives/BP_ReachDestinationObjective.BP_ReachDestinationObjective_C" (Variables|Default|GetConcordTrigger) true "Investigate Concord"))
      (Class|ObjectiveCollection|AddObjective (Class|QuestBase|GetRootObjectiveCollection) _returnvalue_2))
    (:then_2
      (bind _returnvalue_3 (Game|ConstructObjectfromClass "/Game/QuestSystem/Objectives/BP_ReachDestinationObjective.BP_ReachDestinationObjective_C" (Variables|Default|GetDiamondCityTrigger) false "Go to Diamond City"))
      (Class|ObjectiveCollection|AddObjective (Class|QuestBase|GetRootObjectiveCollection) _returnvalue_3))))

(fn ConstructionScript)

(fn ConstructRootObjectiveCollection
  (bind _returnvalue (Game|ConstructObjectfromClass "/Script/QuestSystem.ObjectiveCollection" false true true "Out of Time"))
  (return _returnvalue))