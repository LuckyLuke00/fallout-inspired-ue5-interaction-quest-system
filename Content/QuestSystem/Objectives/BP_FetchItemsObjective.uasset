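; Quest objective that completes when the inventory gains enough of a required item.
; On activation it optionally spawns items at the quest data's spawn points and binds to the inventory's update event.
; When CountItemsAlreadyInInventory is set, it records the starting count and subtracts it, so only newly acquired items count.
; Reaching the target on an inventory update sets the completion flag and fires OnCompleted, while deactivation unbinds the listener.
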(event Custom|OnInventoryUpdated_Event
  (if (CallFunction|HasEnoughItems)
    (Variables|Default|SetEnoughItemsPickedUp true)
    (Class|ObjectiveBase|CallonCompleted self)))

(event EventActivateObjective
  (bind _fetchquestdata (Variables|Default|GetFetchQuestData))
  (|CallParentFunction)
  (Utilities|IsValid (Variables|Default|GetInventoryComponent)
    (:Is%20Valid
      (if (.spawnitem _fetchquestdata)
        (CallFunction|SpawnItems))
      (if (.countitemsalreadyininventory _fetchquestdata)
        (CallFunction|SetInventoryCount))
      (EventDispatchers|AssignOnInventoryUpdated (Variables|Default|GetInventoryComponent) (delegate Custom|OnInventoryUpdated_Event)))
    (:Is%20Not%20Valid
      (Development|PrintString 0 "BP_FetchObjective: Inventory Component is invalid" true true "(R=1.000000,G=0.000000,B=0.000000,A=1.000000)"))))

(event EventDeactivateObjective
  (EventDispatchers|UnbindEventfromOnInventoryUpdated (Variables|Default|GetInventoryComponent) (delegate Custom|OnInventoryUpdated_Event)))

(fn IsComplete
  (return (Variables|Default|GetEnoughItemsPickedUp)))

(fn SpawnItems
  (bind _fetchquestdata (Variables|Default|GetFetchQuestData))
  (for _index (range 0 (- (.amounttofetch _fetchquestdata) 1))
    (if (Utilities|IsValid (Utilities|Array|Get(acopy) (.spawnpoints _fetchquestdata) _index))
      (Default|SpawnActorOfClass (Utilities|Array|Get(acopy) (.spawnpoints _fetchquestdata) _index) (.itemtofetch _fetchquestdata))))
  (return))

(fn SetInventoryCount
  (Variables|Default|SetItemsAlreadyInInventory (Class|InventoryComponent|GetItemCount (Variables|Default|GetInventoryComponent) (.itemtofetch (Variables|Default|GetFetchQuestData))))
  (return))

(fn HasEnoughItems
  (bind _fetchquestdata (Variables|Default|GetFetchQuestData))
  (return (>= (- (Class|InventoryComponent|GetItemCount (Variables|Default|GetInventoryComponent) (.itemtofetch _fetchquestdata)) (Variables|Default|GetItemsAlreadyInInventory)) (.amounttofetch _fetchquestdata))))