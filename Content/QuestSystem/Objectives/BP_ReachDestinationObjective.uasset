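; BP_ReachDestinationObjective is a quest objective that completes when the player character reaches a destination actor.
; On activation it runs the parent logic, then binds to the destination actor's begin-overlap event.
; An overlap by BP_ThirdPersonCharacter unbinds the event, sets DestinationReached and fires OnCompleted with itself.
; IsComplete reports that flag.
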(event Custom|OnActorBeginOverlap_Event
  (params (OverlappedActor :type Actor%20Object%20Reference) (OtherActor :type Actor%20Object%20Reference))
  (Utilities|Casting|CastToBP_ThirdPersonCharacter OtherActor)
  (Collision|UnbindEventfromOnActorBeginOverlap (Variables|Default|GetDesitnation) (delegate Custom|OnActorBeginOverlap_Event))
  (Variables|Default|SetbDestinationReached true)
  (Class|ObjectiveBase|CallonCompleted self))

(event EventActivateObjective
  (|CallParentFunction)
  (EventDispatchers|AssignOnActorBeginOverlap (Variables|Default|GetDesitnation) (delegate Custom|OnActorBeginOverlap_Event)))

(fn IsComplete
  (return (Variables|Default|GetbDestinationReached)))