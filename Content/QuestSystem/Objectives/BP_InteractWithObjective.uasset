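; Quest objective that completes when a chosen actor is interacted with.
; On activation it finds the InteractComponent on ActorToInteractWith, if valid, and binds to its OnInteract event.
; An interaction by any interactor sets HasInteracted, which IsComplete returns, and fires the completed notification.
; Deactivation unbinds the event without rechecking that the component is valid.
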(event Custom|OnInteract_Event
  (params (Interactor :type Actor%20Object%20Reference))
  (Variables|Default|SetbHasInteracted true)
  (Class|ObjectiveBase|CallonCompleted self))

(event EventActivateObjective
  (bind _actortointeractwith (Variables|Default|GetActorToInteractWith))
  (bind _returnvalue (Actor|GetComponentbyClass _actortointeractwith "/Script/QuestSystem.InteractComponent"))
  (|CallParentFunction)
  (Utilities|IsValid _actortointeractwith
    (:Is%20Valid
      (if (Utilities|IsValid _returnvalue)
        (bind _output_get (Variables|Default|SetInteractComponent _returnvalue))
        (EventDispatchers|AssignOnInteract _output_get (delegate Custom|OnInteract_Event))))))

(event EventDeactivateObjective
  (|CallParentFunction)
  (EventDispatchers|UnbindEventfromOnInteract (Variables|Default|GetInteractComponent) (delegate Custom|OnInteract_Event)))

(fn IsComplete
  (return (Variables|Default|GetbHasInteracted)))