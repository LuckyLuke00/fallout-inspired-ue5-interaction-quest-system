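; Quest objective that completes when a player turns in a quest by interacting with a designated actor.
; On activation it binds TryDeliver to the InteractComponent of ActorToDeliver, and unbinds it on deactivation.
; TryDeliver confirms the interactor's QuestManager holds QuestToDeliver, then requires each objective in its root collection, excluding itself, to be complete or optional.
; Success sets IsDelivered, which IsComplete reports, and fires OnCompleted.
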(event Custom|TryDeliver
  (params (Interactor :type Actor%20Object%20Reference))
  (bind _returnvalue (Actor|GetComponentbyClass Interactor "/Script/QuestSystem.QuestManager"))
  (bind _questtodeliver (Variables|Default|GetQuestToDeliver))
  (Utilities|IsValid _returnvalue
    (:Is%20Valid
      (if (Class|QuestManager|HasQuest _returnvalue _questtodeliver)
        (bind _array_element (Utilities|Array|ForEachLoopwithBreak (Class|ObjectiveCollection|GetObjectives (Class|QuestBase|GetRootObjectiveCollection _questtodeliver)) :!label _label)
          (:LoopBody
            (if (!= _array_element self)
              (if (or (CallFunction|IsComplete _array_element) (Class|ObjectiveBase|IsOptional _array_element))
                (Variables|Default|SetbIsDelivered true)
                (else
                  (Variables|Default|SetbIsDelivered false)
                  (goto _label Break)))))
          (:Completed
            (if (Variables|Default|GetbIsDelivered)
              (Class|ObjectiveBase|CallonCompleted self))))))))

(event EventActivateObjective
  (bind _actortodeliver (Variables|Default|GetActorToDeliver))
  (bind _returnvalue (Actor|GetComponentbyClass _actortodeliver "/Script/QuestSystem.InteractComponent"))
  (|CallParentFunction)
  (Utilities|IsValid (Variables|Default|GetQuestToDeliver)
    (:Is%20Valid
      (Utilities|IsValid _actortodeliver
        (:Is%20Valid
          (if (Utilities|IsValid _returnvalue)
            (bind _output_get (Variables|Default|SetInteractComponent _returnvalue))
            (EventDispatchers|AssignOnInteract _output_get (delegate Custom|TryDeliver))))))))

(event EventDeactivateObjective
  (|CallParentFunction)
  (EventDispatchers|UnbindEventfromOnInteract (Variables|Default|GetInteractComponent) (delegate Custom|TryDeliver)))

(fn IsComplete
  (return (Variables|Default|GetbIsDelivered)))